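; BP_randFlickeringLight is an actor whose point light flickers at random intervals.
; The construction script sets the light to its normal Intensity.
; From BeginPlay, a self-restarting loop waits a random delay between Min and Max, then a FlipFlop alternates the light between MinFlickerIntensity and Intensity.
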(event `self.ReceiveBeginPlay`
  (bind _pointlight (`self.PointLight`))
  (`KismetSystemLibrary.RetriggerableDelay` (`KismetMathLibrary.RandomFloatInRange` (`self.Min`) (`self.Max`)) :!label _label)
  (`/Engine/EditorBlueprintResources/StandardMacros.FlipFlop`
    (:`A`
      (`LightComponent.SetIntensity` _pointlight (`self.MinFlickerIntensity`))
      (goto _label))
    (:`B`
      (`LightComponent.SetIntensity` _pointlight (`self.Intensity`))
      (goto _label))))

(fn `UserConstructionScript`
  (`LightComponent.SetIntensity` (`self.PointLight`) (`self.Intensity`)))