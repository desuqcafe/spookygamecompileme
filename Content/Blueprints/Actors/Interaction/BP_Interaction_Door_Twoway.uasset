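; Interactable two-way door Blueprint that toggles open and closed, swinging away from or toward a side chosen by the player's position.
; On opening, it stores the dot product of the player-to-door direction and the mesh's forward vector, whose sign selects positive or negative 90 degrees of yaw.
; A timeline lerps the mesh rotation and reverses to close.
; Tick prints the live dot product for debugging.
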(event `self.Intearct`
  (if (`self.isDoorClosed`)
    (set `self.isDoorClosed` false)
    (set `self.DotProduct` (`KismetMathLibrary.Dot_VectorVector` (`KismetMathLibrary.Normal` (- (`self.K2_GetActorLocation` self) (`self.K2_GetActorLocation` (`self.PlayerRef`)))) (`SceneComponent.GetForwardVector` (`self.StaticMesh`))))
    (bind (_direction _alpha) (`Timeline|OpenDoorTL` :!via `PlayFromStart` :!label _label)
      (:`Update`
        (`SceneComponent.K2_SetRelativeRotation` (`self.StaticMesh`) (`KismetMathLibrary.MakeRotator` 0.0 0.0 (`KismetMathLibrary.Lerp` 0.0 (`KismetMathLibrary.SelectFloat` 90.0 -90.0 (>= (`self.DotProduct`) 0.0)) _alpha)) false false)))
    (else
      (set `self.isDoorClosed` true)
      (goto _label :!via `ReverseFromEnd`))))

(event `self.ReceiveTick`
  (params (DeltaSeconds :type "Float (single-precision)"))
  (`KismetSystemLibrary.PrintString` (`KismetStringLibrary.Conv_DoubleToString` (`KismetMathLibrary.Dot_VectorVector` (`KismetMathLibrary.Normal` (- (`self.K2_GetActorLocation` self) (`self.K2_GetActorLocation` (`self.PlayerRef`)))) (`SceneComponent.GetForwardVector` (`self.StaticMesh`)))) true true (struct :`G` 0.66 :`B` 1.0 :`A` 1.0) DeltaSeconds))

(fn `UserConstructionScript`
  (`parent.UserConstructionScript`))